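; BP_Pawn is a controllable pawn with simple WASD movement and mouse look.
; Mouse input drives controller yaw and inverted pitch, while key presses and releases set forward/back and left/right axis values.
; Tick passes both values to AddMovement, which picks a forward or right vector from control rotation with pitch zeroed, so looking up or down does not tilt movement.
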(event EventTick
  (params (DeltaSeconds :type Float%20%28single-precision%29))
  (Utilities|AddMovement false (Variables|Default|GetFB))
  (Utilities|AddMovement true (Variables|Default|GetLR)))

(event Input|KeyboardEvents|W
  (params (Key :type Key%20Structure :default "None"))
  ;[1 1 1] Simple movement
  (:Pressed
    (Variables|Default|SetFB 1.0))
  (:Released
    (Variables|Default|SetFB 0.0)))

(event Input|KeyboardEvents|A
  (params (Key :type Key%20Structure :default "None"))
  ;[1 1 1] Simple movement
  (:Pressed
    (Variables|Default|SetLR -1.0))
  (:Released
    (Variables|Default|SetLR 0.0)))

(event Input|KeyboardEvents|S
  (params (Key :type Key%20Structure :default "None"))
  ;[1 1 1] Simple movement
  (:Pressed
    (Variables|Default|SetFB -1.0))
  (:Released
    (Variables|Default|SetFB 0.0)))

(event Input|KeyboardEvents|D
  (params (Key :type Key%20Structure :default "None"))
  ;[1 1 1] Simple movement
  (:Pressed
    (Variables|Default|SetLR 1.0))
  (:Released
    (Variables|Default|SetLR 0.0)))

(event Input|MouseEvents|Mouse2D
  (params (AxisValue :type Vector :default "0, 0, 0"))
  ;[1 1 1] Simple movement
  (Pawn|Input|AddControllerYawInput (* (.x AxisValue) 1.0))
  (Pawn|Input|AddControllerPitchInput (* (.y AxisValue) -1.0)))

(fn ConstructionScript)