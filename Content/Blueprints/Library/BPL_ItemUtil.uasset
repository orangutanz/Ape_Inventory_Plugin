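; Blueprint function library of item and inventory helpers for BPC_ApeInventory.
; Looks up item rows in CDT_Items and fetches the inventory component from player pawn 0.
; Adding stages the item, capped at max stack, in the inventory's utility slot, then returns success and that slot's leftover quantity.
; Equip checks match DT_Equipment_Info definitions against the inventory's equipment definitions; FL_FindEquipmentIndex is an empty stub.
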(fn FLGetItemInfo
  (params (ItemID :type Name))
  (bind _returnvalue (Utilities|GetDataTableRow "/Ape_Inventory_Plugin/Data/CDT_Items.CDT_Items" ItemID)
    (:then
      (return _returnvalue true))
    (:RowNotFound
      (return "" false))))

(fn FLFindEquipmentIndex
  (params (DefineName :type Name) (NewParam :type Boolean))
  (return 0 false))

(fn FLGetOwnInventory
  (return (Actor|GetComponentbyClass (Game|Player|GetPlayerPawn 0) "/Ape_Inventory_Plugin/Blueprints/BPC_ApeInventory.BPC_ApeInventory_C")))

(fn FLAddItem
  (params (RefComponent :type Inventory%20Component%20Object%20Reference) (ItemName :type Name) (Quantity :type Integer))
  (LocalVariables|SetTempQuantity Quantity)
  (bind _returnvalue (Class|InventoryComponent|GetUtilitySlot RefComponent))
  (bind _st_item (ItemUtil|FLGetItemInfo ItemName))
  (Class|ItemSlot|SetItemInfo _returnvalue (Utilities|Struct|MakeItemInfo (.ItemID (Utilities|Struct|BreakST_Item _st_item)) (Math|Integer|SelectInt (.MaxStack (Utilities|Struct|BreakST_Item _st_item)) Quantity (> Quantity (.MaxStack (Utilities|Struct|BreakST_Item _st_item)))) (.MaxStack (Utilities|Struct|BreakST_Item _st_item)) (.ItemType (Utilities|Struct|BreakST_Item _st_item))))
  (bind _returnvalue_2 (Class|InventoryComponent|AddItem RefComponent _returnvalue))
  (bind _returnvalue_3 (Class|ItemSlot|GetItemInfo _returnvalue))
  (return _returnvalue_2 (.Quantity (Utilities|Struct|BreakItemInfo _returnvalue_3))))

(fn FLCanEquipItem
  (params (ItemName :type Name) (InventoryRef :type Inventory%20Component%20Object%20Reference))
  (bind _returnvalue (Utilities|GetDataTableRow "/Ape_Inventory_Plugin/Data/Equipment/DT_Equipment_Info.DT_Equipment_Info" ItemName)
    (:then
      (bind _output_get (LocalVariables|SetEquipmentInfo _returnvalue))
      (if (>= (Utilities|Array|FindItem (Variables|/Script/Ape_Inventory.InventoryComponent|GetEquipmentDefinitions InventoryRef) (.Definition (Utilities|Struct|BreakST_EquipmentInfo _output_get))) 0)
        (return (Utilities|Array|FindItem (Variables|/Script/Ape_Inventory.InventoryComponent|GetEquipmentDefinitions InventoryRef) (.Definition (Utilities|Struct|BreakST_EquipmentInfo _output_get))) true)
        (else
          _)))
    (:RowNotFound
      _))
  (return 0 false) ; Target is not an equipment
)