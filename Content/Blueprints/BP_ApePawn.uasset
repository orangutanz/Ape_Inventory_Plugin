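; Player pawn for the Ape inventory system, with WASD and mouse movement, a Tab inventory toggle and E to interact.
; The locally controlled pawn creates its own camera, which smoothly follows CameraTarget and snaps when too far away.
; Each tick a forward sphere trace, shown as a debug sphere, tracks BPI_ApeInventory targets and cancels interaction when the target changes.
; Interactions reach targets through a server event and interface messages.
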(event Custom|SERVER_InteractActor
  (params (TargetActor :type Actor%20Object%20Reference) (toggle :type Boolean))
  ;[1 1 1] Interaction
  (Utilities|IsValid TargetActor
    (:Is%20Valid
      (Class|BPIApeInventory|BPIInteractActor(Message) TargetActor self toggle))))

(event EventBeginPlay
  ;[1 1 1] BeginPlay
  (Private|Initialize))

(event EventTick
  (params (DeltaSeconds :type Float%20%28single-precision%29))
  ;[1 1 1] Tick
  (if (Pawn|IsLocallyControlled)
    (Utilities|AddMovement false (Variables|Control|GetMovementFB))
    (Utilities|AddMovement true (Variables|Control|GetMovementLR))
    (Private|UpdateCamera)))

(event Input|KeyboardEvents|W
  (params (Key :type Key%20Structure :default "None"))
  ;[1 1 1] Simple movement
  (:Pressed
    (Variables|Control|SetMovementFB 1.0))
  (:Released
    (Variables|Control|SetMovementFB 0.0)))

(event Input|KeyboardEvents|A
  (params (Key :type Key%20Structure :default "None"))
  ;[1 1 1] Simple movement
  (:Pressed
    (Variables|Control|SetMovementLR -1.0))
  (:Released
    (Variables|Control|SetMovementLR 0.0)))

(event Input|KeyboardEvents|S
  (params (Key :type Key%20Structure :default "None"))
  ;[1 1 1] Simple movement
  (:Pressed
    (Variables|Control|SetMovementFB -1.0))
  (:Released
    (Variables|Control|SetMovementFB 0.0)))

(event Input|KeyboardEvents|D
  (params (Key :type Key%20Structure :default "None"))
  ;[1 1 1] Simple movement
  (:Pressed
    (Variables|Control|SetMovementLR 1.0))
  (:Released
    (Variables|Control|SetMovementLR 0.0)))

(event Input|KeyboardEvents|Tab
  (params (Key :type Key%20Structure :default "None"))
  (bind _bpc_apeinventory (Variables|Default|GetBPC_ApeInventory))
  ;[1 1 1] Toggle widget
  (:Pressed
    (bind _isinviewport (Default|GetInventoryWidget _bpc_apeinventory))
    (Default|ToggleWidget _bpc_apeinventory (not _isinviewport))))

(event Input|KeyboardEvents|E
  (params (Key :type Key%20Structure :default "None"))
  (bind _lookattargets (Variables|Default|GetLookAtTargets))
  (bind _output (Utilities|ResolveSoftReference _lookattargets))
  ;[1 1 1] Interaction
  (:Pressed
    (Utilities|Casting|CastToBPI_ApeInventory _output)
    (bind (_widgetref _isinviewport) (Default|GetInventoryWidget (Variables|Default|GetBPC_ApeInventory)))
    (Class|BPIApeInventory|BPIToggleInteraction(Message) _widgetref (not _isinviewport))
    (CallFunction|SERVERInteractActor _output (not _isinviewport))))

(event Input|MouseEvents|Mouse2D
  (params (AxisValue :type Vector :default "0, 0, 0"))
  ;[1 1 1] Simple movement
  (Pawn|Input|AddControllerYawInput (* (.x AxisValue) 1.0))
  (Pawn|Input|AddControllerPitchInput (* (.y AxisValue) -1.0)))

(fn ConstructionScript)

(fn Initialize
  (if (Pawn|IsLocallyControlled)
    (Actor|Tick|SetActorTickEnabled true)
    (bind _returnvalue (Game|AddComponentbyClass "/Script/Engine.CameraComponent" true (Transformation|GetWorldTransform (Variables|Default|GetCameraTarget))))
    (Variables|Default|SetCamera _returnvalue)))

(fn UpdateCamera
  (bind _returnvalue (Utilities|Time|GetWorldDeltaSeconds))
  (bind _returnvalue_2 (Utilities|Time|GetWorldDeltaSeconds))
  (bind _returnvalue_3 (Transformation|GetActorForwardVector))
  (bind _camera (Variables|Default|GetCamera))
  (bind _cameratarget (Variables|Default|GetCameraTarget))
  (bind _camera_2 (Variables|Default|GetCamera))
  (bind _returnvalue_4 (Transformation|GetWorldLocation _camera))
  (bind _returnvalue_5 (Transformation|GetWorldLocation _cameratarget))
  (bind _returnvalue_6 (Transformation|GetWorldLocation _camera_2))
  (Utilities|FlowControl|Sequence
    (:then_0
      ;[1 1 1] Update location
      (Transformation|SetWorldLocationAndRotation (Variables|Default|GetCamera) (select (> (Class|KismetMathLibrary|VectorDistanceSquared _returnvalue_4 _returnvalue_5) 9999999.0) _returnvalue_5 (Math|Interpolation|VInterpTo _returnvalue_4 _returnvalue_5 _returnvalue_2 12.0)) (Math|Interpolation|RInterpTo (Transformation|GetWorldRotation _camera) (Transformation|GetWorldRotation _cameratarget) _returnvalue_2 24.0) false false))
    (:then_1
      ;[1 1 1] Update target
      (bind _outhit (Collision|SphereTraceByChannel (+ _returnvalue_6 (* _returnvalue_3 6e+01)) (+ _returnvalue_6 (* _returnvalue_3 6.5e+02)) 8.0 "TraceTypeQuery1" false 0 "None"))
      (Rendering|Debug|DrawDebugSphere (Math|Vector|SelectVector (.ImpactPoint (Collision|BreakHitResult _outhit)) (.TraceEnd (Collision|BreakHitResult _outhit)) (.bBlockingHit (Collision|BreakHitResult _outhit))) 8.0 2 (Math|Color|SelectColor "(R=0.000000,G=1.000000,B=0.000000,A=1.000000)" "(R=1.000000,G=1.000000,B=1.000000,A=1.000000)" (.bBlockingHit (Collision|BreakHitResult _outhit))) (+ _returnvalue _returnvalue) 1.0)
      ;[1 1 1] Update interaction on different target
      (if (.bBlockingHit (Collision|BreakHitResult _outhit))
        (if (not (== (Utilities|ResolveSoftReference (Variables|Default|GetLookAtTargets)) (.HitActor (Collision|BreakHitResult _outhit))))
          (Class|BPIApeInventory|BPIToggleInteraction(Message) (Utilities|ResolveSoftReference (Variables|Default|GetLookAtTargets)) false)
          (CallFunction|SERVERInteractActor (Utilities|ResolveSoftReference (Variables|Default|GetLookAtTargets)) false)
          (Variables|Default|SetLookAtTargets 0)
          (Utilities|Casting|CastToBPI_ApeInventory (.HitActor (Collision|BreakHitResult _outhit)))
          (Variables|Default|SetLookAtTargets (Utilities|ResolveSoftReference (.HitActor (Collision|BreakHitResult _outhit)))))
        (else
          (if (Utilities|IsValidSoftObjectReference (Variables|Default|GetLookAtTargets))
            (Class|BPIApeInventory|BPIToggleInteraction(Message) (Utilities|ResolveSoftReference (Variables|Default|GetLookAtTargets)) false)
            (CallFunction|SERVERInteractActor (Utilities|ResolveSoftReference (Variables|Default|GetLookAtTargets)) false))
          (Variables|Default|SetLookAtTargets 0))))))

(fn ToggleInputMode)