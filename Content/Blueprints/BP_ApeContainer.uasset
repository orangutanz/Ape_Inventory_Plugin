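; BP_ApeContainer is an interactable loot container with a hinged lid and an inventory whose size and starting items are randomized on the server.
; Interacting actors are tracked in a list that drives Opening, whose OnRep starts a looping timer easing the lid toward open or closed until it settles.
; Toggling interaction registers the container as the player's viewed inventory and adds or removes its widget in the player's inventory screen.
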(event Custom|BoxAnim
  (bind _tophinge (Variables|Default|GetTopHinge))
  (bind _opening (Variables|Default|GetOpening))
  (bind _returnvalue (Math|Float|SelectFloat 45.0 0.0 _opening))
  (bind _relativerotation (Variables|/Script/Engine.SceneComponent|GetRelativeRotation _tophinge))
  ;[1 1 1] Interaction
  (Transformation|SetRelativeRotation _tophinge (Math|Rotator|MakeRotator 0.0 (Math|Interpolation|FInterpTo (.pitch _relativerotation) _returnvalue 0.03 8.0) 0.0) false false)
  (if (Math|Float|NearlyEqual(Float) (.pitch _relativerotation) _returnvalue 0.01)
    (Utilities|Time|PauseTimerbyHandle (Variables|Default|GetAnimHandle))
    (Utilities|Time|ClearandInvalidateTimerbyHandle (Variables|Default|GetAnimHandle))
    (Variables|Default|SetAnimHandle "")))

(event EventBPIToggleInteraction
  (params (Toggle :type Boolean))
  ;[1 1 1] Interaction
  (CallFunction|ToggleInventory Toggle))

(event EventBPIInteractActor
  (params (FromWhom :type Pawn%20Object%20Reference) (toggle :type Boolean))
  (bind _output (Utilities|ResolveSoftReference FromWhom))
  (bind _interactinglist (Variables|Default|GetInteractingList))
  ;[1 1 1] Interaction
  (if toggle
    (Utilities|Array|AddUnique _interactinglist _output)
    (else
      (Utilities|Array|RemoveItem _interactinglist _output)))
  (Variables|Default|SetOpening (Utilities|Array|IsNotEmpty _interactinglist)))

(event EventBeginPlay
  ;[1 1 1] Intial random items
  (if (Networking|IsServer)
    (bind _outrownames (DataTable|GetDataTableRowNames "/Ape_Inventory_Plugin/Data/CDT_Items.CDT_Items"))
    (for _index (range 0 (Math|Random|RandomIntegerinRange 5 12))
      (CallFunction|FLAddItem (Variables|Default|GetBPC_ApeInventory) (.OutItem (Utilities|Array|Random _outrownames)) (Math|Random|RandomIntegerinRange 1 6)))))

(fn ConstructionScript
  (if (Networking|IsServer)
    (Variables|/Script/Ape_Inventory.InventoryComponent|SetInventorySize (Variables|Default|GetBPC_ApeInventory) (* (Math|Random|RandomIntegerinRange 2 5) 5))))

(fn ToggleInventory
  (params (Toggle :type Boolean))
  (bind _inventoryref (CallFunction|FLGetOwnInventory))
  (Utilities|FlowControl|Sequence
    (:then_0
      (bind (_widgetref _isinviewport) (Default|GetInventoryWidget _inventoryref))
      (bind _aswbp_player_inventory (Utilities|Casting|CastToWBP_PlayerInventory _widgetref))
      (bind _widgetref_2 (Default|GetInventoryWidget (Variables|Default|GetBPC_ApeInventory))))
    (:then_1
      (Class|InventoryComponent|GetViewInventory _inventoryref (Variables|Default|GetBPC_ApeInventory) true)
      (if Toggle
        (if _isinviewport
          _
          (else
            (Default|ToggleWidget _inventoryref true)))
        (Default|AddViewingWidget _aswbp_player_inventory _widgetref_2)
        (else
          (Default|ToggleWidget _inventoryref false)
          (Default|RemoveViewingWidget _aswbp_player_inventory _widgetref_2))))))

(fn OnRepOpening
  (if (Utilities|Time|IsValidTimerHandle (Variables|Default|GetAnimHandle))
    (Utilities|Time|UnpauseTimerbyHandle (Variables|Default|GetAnimHandle))
    (else
      (bind _returnvalue (Utilities|Time|SetTimerbyEvent (EventDispatchers|CreateEvent :!event Custom|BoxAnim) 0.03 true))
      (Variables|Default|SetAnimHandle _returnvalue))))

(fn BPIGetInventory
  (return 0))