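; Inventory component that adds an on-screen inventory widget to its parent class.
; BeginPlay async-loads the widget class, creates the widget and passes it the component through an interface message.
; GetInventoryWidget returns that widget or builds one by blocking load without that message; ToggleWidget uses it to switch viewport display, cursor and input mode.
; Unwired Client, Server and Utility nodes lay out inventory and equipment calls but never run.
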(event EventBeginPlay
  (|CallParentFunction)
  (bind _class (Utilities|AsyncLoadClassAsset (Variables|Ape_Inventory|GetWidgetClass))
    (:Completed
      (bind _asuser_widget (Utilities|Casting|CastToUserWidgetClass _class))
      (bind _returnvalue (UserInterface|CreateWidget _asuser_widget))
      (bind _output_get (Variables|Default|SetWB_InventoryRef _returnvalue))
      (Class|BPIApeInventory|BPISetInventory(Message) _output_get self))))

(fn ToggleWidget
  (params (Toggle :type Boolean))
  (bind _returnvalue (Game|GetPlayerController 0))
  (bind _widgetref (Public|GetInventoryWidget))
  (Utilities|IsValid _widgetref
    (:Is%20Valid
      (Utilities|FlowControl|Sequence
        (:then_0
          (if Toggle
            (UserInterface|Viewport|AddtoViewport _widgetref 0)
            (else
              (Widget|RemovefromParent _widgetref))))
        (:then_1
          (bind _output_get (Variables|/Script/Engine.PlayerController|SetbShowMouseCursor (Game|GetPlayerController 0) Toggle))
          (if _output_get
            (Input|SetInputModeGameandUI _returnvalue 0 "DoNotLock" true false)
            (else
              (Input|SetInputModeGameOnly _returnvalue false))))))))

(fn GetInventoryWidget
  (Utilities|IsValid (Variables|Default|GetWB_InventoryRef)
    (:Is%20Valid
      _)
    (:Is%20Not%20Valid
      (bind _returnvalue (Utilities|LoadClassAssetBlocking (Variables|Ape_Inventory|GetWidgetClass)))
      (bind _asuser_widget (Utilities|Casting|CastToUserWidgetClass _returnvalue))
      (bind _returnvalue_2 (UserInterface|CreateWidget _asuser_widget))
      (Variables|Default|SetWB_InventoryRef _returnvalue_2)))
  (return (Variables|Default|GetWB_InventoryRef) (UserInterface|Viewport|IsinViewport (Variables|Default|GetWB_InventoryRef))))