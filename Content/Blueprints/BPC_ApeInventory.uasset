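; Inventory component that extends a parent inventory class with a UI widget and world item drops.
; BeginPlay async-loads and creates the widget, passes it the component, and binds the drop event; GetInventoryWidget falls back to a blocking load.
; ToggleWidget switches viewport display, cursor and input mode, while HandleDropItem spawns a pickup ahead of the owner.
; Access level defers to the parent, and unwired nodes catalogue the inherited inventory API.
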(event EventBeginPlay
  (|CallParentFunction)
  (Utilities|FlowControl|Sequence
    (:then_0
      (bind _class (Utilities|AsyncLoadClassAsset (Variables|Ape_Inventory|GetWidgetClass))
        (:Completed
          (bind _asuser_widget (Utilities|Casting|CastToUserWidgetClass _class))
          (bind _returnvalue (UserInterface|CreateWidget _asuser_widget))
          (bind _output_get (Variables|Default|SetWB_InventoryRef _returnvalue))
          (Class|BPIApeInventory|BPISetInventory(Message) _output_get self))))
    (:then_1
      (EventDispatchers|AssignOnDropInventoryItem (EventDispatchers|CreateEvent :!event HandleDropItem)))))

(fn ToggleWidget
  (params (Toggle :type Boolean))
  (bind _returnvalue (Game|GetPlayerController 0))
  (bind _widgetref (Public|GetInventoryWidget))
  (Utilities|IsValid _widgetref
    (:Is%20Valid
      (Utilities|FlowControl|Sequence
        (:then_0
          (if Toggle
            (UserInterface|Viewport|AddtoViewport _widgetref 0)
            (else
              (Widget|RemovefromParent _widgetref))))
        (:then_1
          (bind _output_get (Variables|/Script/Engine.PlayerController|SetbShowMouseCursor (Game|GetPlayerController 0) Toggle))
          (if _output_get
            (Input|SetInputModeGameandUI _returnvalue 0 "DoNotLock" true false)
            (else
              (Input|SetInputModeGameOnly _returnvalue false))))))))

(fn GetInventoryWidget
  (Utilities|IsValid (Variables|Default|GetWB_InventoryRef)
    (:Is%20Valid
      _)
    (:Is%20Not%20Valid
      (bind _returnvalue (Utilities|LoadClassAssetBlocking (Variables|Ape_Inventory|GetWidgetClass)))
      (bind _asuser_widget (Utilities|Casting|CastToUserWidgetClass _returnvalue))
      (bind _returnvalue_2 (UserInterface|CreateWidget _asuser_widget))
      (Variables|Default|SetWB_InventoryRef _returnvalue_2)))
  (return (Variables|Default|GetWB_InventoryRef) (UserInterface|Viewport|IsinViewport (Variables|Default|GetWB_InventoryRef))))

(fn GetAccessLevel
  (params (TargetInventory :type Inventory%20Component%20Object%20Reference))
  (bind _returnvalue (|CallParentFunction TargetInventory)) ; Default unlimited access
  (return _returnvalue))

(fn HandleDropItem
  (params (itemInfo :type Item%20Info%20Structure))
  (bind _returnvalue (Components|GetOwner))
  (bind _returnvalue_2 (Game|SpawnActorfromClass "/Ape_Inventory_Plugin/Blueprints/BP_Ape_Item_Pickup.BP_Ape_Item_Pickup_C" (Math|Transform|MakeTransform (+ (+ (.location (Transformation|GetActorTransform _returnvalue)) "0.000000,0.000000,60.000000") (* (Transformation|GetActorForwardVector _returnvalue) (Math|Random|RandomFloatinRange 5e+01 9e+01))) "0, 0, 0" "1.000000,1.000000,1.000000") "AdjustIfPossibleButAlwaysSpawn" 0 itemInfo 0)))