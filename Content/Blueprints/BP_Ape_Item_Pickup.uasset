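; BP_Ape_Item_Pickup is a physics-simulated world item that actors with an InventoryComponent pick up by interacting.
; InitializeItem runs at construction and BeginPlay, looking up ItemInfo's ID and blocking-loading its mesh and materials.
; A missing mesh shrinks the component; an empty material list puts the item icon on a dynamic material.
; Interaction passes ItemInfo through the inventory's utility slot, destroying the pickup when fully added, otherwise retaining the remainder.
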(event EventBeginPlay
  (CallFunction|InitializeItem false))

(event EventBPIInteractActor
  (params (FromWhom :type Pawn%20Object%20Reference) (toggle :type Boolean))
  (bind _returnvalue (Actor|GetComponentbyClass FromWhom "/Script/Ape_Inventory.InventoryComponent"))
  (if toggle
    (if (Utilities|IsValid self)
      (Utilities|IsValid _returnvalue
        (:Is%20Valid
          (bind _returnvalue_2 (Class|InventoryComponent|GetUtilitySlot _returnvalue))
          (Class|ItemSlot|SetItemInfo _returnvalue_2 (Variables|Default|GetItem_Info))
          (bind _returnvalue_3 (Class|InventoryComponent|AddItem _returnvalue _returnvalue_2))
          (if _returnvalue_3
            (Actor|DestroyActor) ; Fully added
            (else
              (bind _returnvalue_4 (Class|ItemSlot|GetItemInfo _returnvalue_2)) ; Partially Added or Not Added
              (Variables|Default|SetItem_Info _returnvalue_4))))))))

(fn ConstructionScript
  (CallFunction|InitializeItem true))

(fn InitializeItem
  (params (bConstructionScript :type Boolean))
  (bind _staticmesh (Variables|Default|GetStaticMesh))
  (if bConstructionScript
    _
    (else
      _))
  (Physics|SetSimulatePhysics (Variables|Default|GetStaticMesh) true)
  (bind _st_item (CallFunction|FLGetItemInfo (.ItemID (Utilities|Struct|BreakItemInfo (Variables|Default|GetItem_Info)))))
  (Utilities|FlowControl|Sequence
    (:then_0
      (bind _returnvalue (Utilities|LoadAssetBlocking (.Mesh (Utilities|Struct|BreakST_Item _st_item))))
      (bind _asstatic_mesh (Utilities|Casting|CastToStaticMesh _returnvalue)
        (:then
          (Components|StaticMesh|SetStaticMesh _staticmesh _asstatic_mesh))
        (:CastFailed
          (Transformation|SetWorldScale3D _staticmesh "0.250000,0.250000,0.250000"))))
    (:then_1
      (if (Utilities|Array|IsEmpty (.Materials (Utilities|Struct|BreakST_Item _st_item)))
        (bind _returnvalue_2 (Utilities|LoadAssetBlocking (.Icon (Utilities|Struct|BreakST_Item _st_item))))
        (bind _astexture_2d (Utilities|Casting|CastToTexture2D _returnvalue_2))
        (bind _returnvalue_3 (Rendering|Material|CreateDynamicMaterialInstance _staticmesh 0 "/Ape_Inventory_Plugin/Material/MI_PickUp.MI_PickUp" "None" :!class /Script/Engine.PrimitiveComponent))
        (Rendering|Material|SetTextureParameterValue _returnvalue_3 "Texture" _astexture_2d)
        (Rendering|Material|SetMaterial _staticmesh 0 _returnvalue_3)
        (else
          (for (_array_element _array_index) (.Materials (Utilities|Struct|BreakST_Item _st_item))
            (bind _returnvalue_4 (Utilities|LoadAssetBlocking _array_element))
            (bind _asmaterial_instance (Utilities|Casting|CastToMaterialInstance _returnvalue_4))
            (Rendering|Material|SetMaterial (Variables|Default|GetStaticMesh) _array_index _asmaterial_instance)))))))

(fn BPIGetInventory
  (return 0))