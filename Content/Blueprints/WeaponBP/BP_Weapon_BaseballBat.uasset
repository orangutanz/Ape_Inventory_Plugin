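; Baseball bat weapon Blueprint that plays a procedural swing when used, with no hit or damage logic in its graphs.
; A server interact press multicasts the swing unless one is already in its forward stroke.
; A looping timer interpolates the Handle's pitch down quickly, then back to rest more slowly, deriving sideways offset from pitch.
; The timer pauses at rest and is reused for later swings, leaving Tick unused.
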(event Custom|MULTICAST_Swing
  (Variables|Default|SetSwinging true)
  (Transformation|SetRelativeRotation (Variables|Default|GetHandle) "0, 0, 0" false false)
  (if (Utilities|Time|IsValidTimerHandle (Variables|Default|GetSwingAnimHandle))
    (Utilities|Time|UnpauseTimerbyHandle (Variables|Default|GetSwingAnimHandle))
    (else
      (bind _returnvalue (Utilities|Time|SetTimerbyEvent (delegate Custom|CE_SwingAnim) 0.03 true))
      (Variables|Default|SetSwingAnimHandle _returnvalue))))

(event Custom|CE_SwingAnim
  (bind _handle (Variables|Default|GetHandle))
  (bind _relativerotation (Variables|/Script/Engine.SceneComponent|GetRelativeRotation _handle))
  (Transformation|SetRelativeLocationAndRotation _handle (Math|Vector|MakeVector 0.0 (* (Math|Interpolation|FInterpTo (.pitch _relativerotation) (Math|Float|SelectFloat -9e+01 0.0 (Variables|Default|GetSwinging)) 0.03 (Math|Float|SelectFloat 14.0 8.0 (Variables|Default|GetSwinging))) -0.33) 0.0) (Math|Rotator|MakeRotator 0.0 (Math|Interpolation|FInterpTo (.pitch _relativerotation) (Math|Float|SelectFloat -9e+01 0.0 (Variables|Default|GetSwinging)) 0.03 (Math|Float|SelectFloat 14.0 8.0 (Variables|Default|GetSwinging))) 0.0) false false)
  (if (Variables|Default|GetSwinging)
    (if (Math|Float|NearlyEqual(Float) (.pitch _relativerotation) -9e+01 0.5)
      (Variables|Default|SetSwinging false))
    (elif (Math|Float|NearlyEqual(Float) (.pitch _relativerotation) 0.0 0.2)
      (Utilities|Time|PauseTimerbyHandle (Variables|Default|GetSwingAnimHandle)))))

(event EventBeginPlay
  (|CallParentFunction) ; This node is disabled and will not be called.\nDrag off pins to build functionality.
)

(event Collision|EventActorBeginOverlap
  (params (OtherActor :type Actor%20Object%20Reference))
  (|CallParentFunction OtherActor) ; This node is disabled and will not be called.\nDrag off pins to build functionality.
)

(event EventTick
  (params (DeltaSeconds :type Float%20%28single-precision%29))
  (|CallParentFunction DeltaSeconds) ; This node is disabled and will not be called.\nDrag off pins to build functionality.
)

(event EventBPIInteractonServer
  (params (FromWhom :type Pawn%20Object%20Reference) (toggle :type Boolean))
  (if toggle
    (if (not (Variables|Default|GetSwinging))
      (CallFunction|MULTICASTSwing))))

(fn ConstructionScript
  (|CallParentFunction))